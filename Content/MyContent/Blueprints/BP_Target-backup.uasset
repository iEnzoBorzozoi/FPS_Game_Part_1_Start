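; Target actor that moves in a repeating path and takes hits until it explodes and is destroyed.
; Four chained timelines apply local offsets to SMTarget along BaseDirection, ModifiedDirection, then both negated, before restarting the first.
; Hit decrements HitPoints and spawns small impact effects and sound, or larger destruction ones at zero.
; Older timer, world-offset and timeline-reversal movement logic remains disconnected.
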(event `self.ReceiveBeginPlay`
  ; LoopingMovement
  (bind (_direction _move1) (`Timeline|Timeline` :!label _label)
    (:`Update`
      (`SceneComponent.K2_AddLocalOffset` (`self.SM_Target`) (`KismetMathLibrary.VLerp` (0.0 0.0 0.0) (`self.BaseDirection`) _move1) false false))
    (:`Finished`
      (bind (_direction_2 _move2) (`Timeline|Timeline_0` :!via `PlayFromStart`)
        (:`Update`
          (`SceneComponent.K2_AddLocalOffset` (`self.SM_Target`) (`KismetMathLibrary.VLerp` (0.0 0.0 0.0) (`self.ModifiedDirection`) _move2) false false))
        (:`Finished`
          (bind (_direction_3 _move1_2) (`Timeline|Timeline_1` :!via `PlayFromStart`)
            (:`Update`
              (`SceneComponent.K2_AddLocalOffset` (`self.SM_Target`) (`KismetMathLibrary.VLerp` (0.0 0.0 0.0) (* (`self.BaseDirection`) -1.0) _move1_2) false false))
            (:`Finished`
              (bind (_direction_4 _move2_2) (`Timeline|Timeline_2` :!via `PlayFromStart`)
                (:`Update`
                  (`SceneComponent.K2_AddLocalOffset` (`self.SM_Target`) (`KismetMathLibrary.VLerp` (0.0 0.0 0.0) (* (`self.ModifiedDirection`) -1.0) _move2_2) false false))
                (:`Finished`
                  (`self.restartMove1`))))))))))

(event `restartMove1`
  ; LoopingMovement
  (goto _label :!via `PlayFromStart`))

(event `Event_FlipDirection`
  ;[1 0.3095 0] flip direction
  (set `self.CurrentDirection` (* (`self.CurrentDirection`) -1.0)))

(event `reverseMove1`
  ; LoopingMovement
  (goto _label :!via `Reverse`))

(event `Event_ChangeDirection`
  ;[1 0.3095 0] flip direction
  (set `self.CurrentDirection` (`self.ModifiedDirection`)))

(event `Event_ResetDirection`
  ;[1 0.3095 0] flip direction
  (set `self.CurrentDirection` (`self.BaseDirection`)))

(event `self.ReceiveTick`
  (params (DeltaSeconds :type "Float (single-precision)"))
  ;[0 1 0.8838] move
)

(event `self.ReceiveHit`
  (params (MyComp :type "PrimitiveComponent Object Reference") (Other :type "Actor Object Reference") (OtherComp :type "PrimitiveComponent Object Reference") (bSelfMoved :type Boolean) (HitLocation :type "Vector Structure") (HitNormal :type "Vector Structure") (NormalImpulse :type "Vector Structure") (Hit :type "HitResult Structure (by ref)"))
  (bind _hitpoints (`self.HitPoints`))
  ; targHit
  (set `self.HitPoints` (- _hitpoints 1))
  (if (<= _hitpoints 0)
    ; Targ dest
    (bind _output_get (set `self.System Template` (`self.System Template`)))
    (`NiagaraFunctionLibrary.SpawnSystemAtLocation` _output_get HitLocation)
    (`GameplayStatics.SpawnSoundAtLocation` "/Game/MyContent/Audio/MP3_Explosion_Big.MP3_Explosion_Big" HitLocation (struct) 1.0 1.0 0.0 null null)
    (`self.K2_DestroyActor`)
    (else
      (`NiagaraFunctionLibrary.SpawnSystemAtLocation` "/Game/MyContent/FX/PE_Target_Hit.PE_Target_Hit" HitLocation)
      (`GameplayStatics.SpawnSoundAtLocation` "/Game/MyContent/Audio/MP3_Explosions_Small.MP3_Explosions_Small" HitLocation (struct) 1.0 1.0 0.0 null null))))

(fn `UserConstructionScript`)
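; BP_EnergyBooster is a pickup that recharges the first-person player's flashlight energy.
; It caches the player character on BeginPlay and reacts when that character overlaps its Collision component.
; If flashlight energy is below max, it adds ENChargeValue without clamping, plays a collect sound at the cylinder mesh and destroys itself.
; At full energy the pickup stays in the world.
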(event `self.ReceiveBeginPlay`
  ; setup
  (bind _asbp_first_person_character (cast `/Game/StarterContent/FirstPerson/Blueprints/BP_FirstPersonCharacter` (`GameplayStatics.GetPlayerCharacter` 0)))
  (set `self.player ref` _asbp_first_person_character))

(event `self.collision.OnComponentBeginOverlap`
  (params (OverlappedComponent :type "PrimitiveComponent Object Reference") (OtherActor :type "Actor Object Reference") (OtherComp :type "PrimitiveComponent Object Reference") (OtherBodyIndex :type Integer) (bFromSweep :type Boolean) (SweepResult :type "HitResult Structure (by ref)"))
  (bind _player_ref (`self.player ref`))
  (bind _flashlight_en_current (`/Game/StarterContent/FirstPerson/Blueprints/BP_FirstPersonCharacter.Flashlight_EN_Current` _player_ref))
  ; EN booster
  (if (== OtherActor _player_ref)
    (if (< _flashlight_en_current (`/Game/StarterContent/FirstPerson/Blueprints/BP_FirstPersonCharacter.Flashlight_EN_Max` _player_ref))
      (set `/Game/StarterContent/FirstPerson/Blueprints/BP_FirstPersonCharacter.Flashlight_EN_Current` (+ _flashlight_en_current (`self.EN_ChargeValue`)) _player_ref)
      (`GameplayStatics.PlaySoundAtLocation` "/Game/MyContent/Audio/MP3_Key_Collect.MP3_Key_Collect" (`SceneComponent.K2_GetComponentLocation` (`self.SM_Cylinder`)) (struct) 1.0 1.0 0.0 null null null null)
      (`self.K2_DestroyActor`))))

(fn `UserConstructionScript`)
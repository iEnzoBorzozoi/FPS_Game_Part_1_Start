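; BP_LevelTrans is a trigger that moves the player between levels or marks them as escaped.
; BeginPlay caches the first-person character, and the Collision overlap reacts only to that actor.
; In FirstPersonMap it opens StealthMap and briefly disables input around a delay.
; In any other map it sets the character's Escaped flag and disables input without restoring it.
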(event `self.ReceiveBeginPlay`
  ; setup
  (bind _asbp_first_person_character (cast `/Game/StarterContent/FirstPerson/Blueprints/BP_FirstPersonCharacter` (`GameplayStatics.GetPlayerCharacter` 0)))
  (set `self.PlayerRef` _asbp_first_person_character))

(event `self.collision.OnComponentBeginOverlap`
  (params (OverlappedComponent :type "PrimitiveComponent Object Reference") (OtherActor :type "Actor Object Reference") (OtherComp :type "PrimitiveComponent Object Reference") (OtherBodyIndex :type Integer) (bFromSweep :type Boolean) (SweepResult :type "HitResult Structure (by ref)"))
  (bind _returnvalue (`GameplayStatics.GetPlayerController` 0))
  (bind _playerref (`self.PlayerRef`))
  (bind _playerref_2 (`self.PlayerRef`))
  ; Level transitioning
  (if (== OtherActor _playerref)
    (bind _returnvalue_2 (`GameplayStatics.GetCurrentLevelName` true))
    (if (`KismetStringLibrary.EqualEqual_StrStr` _returnvalue_2 "FirstPersonMap")
      (`GameplayStatics.OpenLevel` "StealthMap")
      (`self.DisableInput` _playerref_2 _returnvalue)
      (`KismetSystemLibrary.Delay` 1.0)
      (`self.EnableInput` _playerref_2 _returnvalue)
      (else
        (set `/Game/StarterContent/FirstPerson/Blueprints/BP_FirstPersonCharacter.escaped` true _playerref)
        (`self.DisableInput` _playerref (`PlayerState.GetPlayerController` (`Pawn.PlayerState` _playerref)))))))

(fn `UserConstructionScript`)
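; BP_Camera is a security camera that sweeps between two rotations and catches the first-person player.
; A looping FlipFlop alternates the target rotation, moves the camera mesh to it and repeats after a delay.
; Each tick, a debug-drawn multi line trace runs forward from SMLineTrace, and hitting the player sets Caught and disables input.
; The StealthMap reload is unconnected, so it never runs.
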(event `self.ReceiveBeginPlay`
  (`self.Move_Camera`)
  (bind _asbp_first_person_character (cast `/Game/StarterContent/FirstPerson/Blueprints/BP_FirstPersonCharacter` (`GameplayStatics.GetPlayerCharacter` 0)))
  (set `self.PlayerRef` _asbp_first_person_character))

(event `Move_Camera`
  (bind (_currentrotation_x _currentrotation_y _currentrotation_z) (`KismetMathLibrary.BreakVector` (`self.CurrentRotation`)))
  ; move camera
  (`/Engine/EditorBlueprintResources/StandardMacros.FlipFlop`
    (:`A`
      (set `self.CurrentRotation` (`self.EndRotation`)))
    (:`B`
      (set `self.CurrentRotation` (`self.BaseRotation`))))
  (`KismetSystemLibrary.MoveComponentTo` (`self.SM_Camera`) (0.0 0.0 0.0) (`KismetMathLibrary.MakeRotator` _currentrotation_x _currentrotation_y _currentrotation_z) false false (`self.Speed`))
  (`KismetSystemLibrary.Delay` (`self.Delay`))
  (`self.Move_Camera`))

(event `self.ReceiveTick`
  (params (DeltaSeconds :type "Float (single-precision)"))
  (`self.detect`))

(event `detect`
  (bind _playerref (`self.PlayerRef`))
  (bind _sm_linetrace (`self.SM_LineTrace`))
  (bind _returnvalue (`SceneComponent.K2_GetComponentLocation` _sm_linetrace))
  ; cam detect\
  (bind _outhits (`KismetSystemLibrary.LineTraceMulti` :`Start` _returnvalue :`End` (+ _returnvalue (* (`KismetMathLibrary.GetForwardVector` (`SceneComponent.K2_GetComponentRotation` _sm_linetrace)) (`self.DetectRange`))) :`TraceChannel` "TraceTypeQuery2" :`DrawDebugType` "ForOneFrame"))
  (for _array_element _outhits
    (if (== (`.HitActor` (`GameplayStatics.BreakHitResult` _array_element)) (`self.PlayerRef`))
      (set `/Game/StarterContent/FirstPerson/Blueprints/BP_FirstPersonCharacter.Caught` true (`self.PlayerRef`))
      (`self.DisableInput` _playerref (`PlayerState.GetPlayerController` (`Pawn.PlayerState` _playerref)))
      (`KismetSystemLibrary.Delay` 1.0))))

(fn `UserConstructionScript`)